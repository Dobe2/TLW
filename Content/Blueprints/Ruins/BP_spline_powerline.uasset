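; Spline-placed powerline that builds a row of poles linked by two cables each, entirely in the construction script.
; It spawns a BP_powerline child actor at every spline point, matching the point's rotation, and collects them in an array.
; A second pass snaps each pole's cables to the next pole's connections, sizing them to that distance plus random slack.
; The final pole's cables are set to zero length.
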(event EventBeginPlay)

(event Collision|EventActorBeginOverlap
  (params (OtherActor :type Actor%20Object%20Reference)))

(event EventTick
  (params (DeltaSeconds :type Float%20%28single-precision%29)))

(fn ConstructionScript
  (bind _spline (Variables|Default|GetSpline))
  (bind _output_get (Variables|Default|SetNumberOfSplinePoints (- (Spline|GetNumberOfSplinePoints (Variables|Default|GetSpline)) 1)))
  (for _index (range 0 _output_get)
    (Variables|Default|SetIndexOfLoop _index)
    (bind _returnvalue (AddComponent|AddChildActorComponent false (Math|Conversions|ToTransform(Vector) (Spline|GetLocationatSplinePoint _spline (Variables|Default|GetIndexOfLoop) "Local"))))
    (ChildActorComponent|SetChildActorClass _returnvalue "/Game/Blueprints/Ruins/BP_powerline.BP_powerline_C")
    (bind _asbp_powerline (Utilities|Casting|CastToBP_powerline (Variables|/Script/Engine.ChildActorComponent|GetChildActor _returnvalue)))
    (Utilities|Array|Add (Variables|Default|GetAllChildActorsOfPowerline) _asbp_powerline)
    (Transformation|SetRelativeRotation _returnvalue (Spline|GetRotationatSplinePoint _spline (Variables|Default|GetIndexOfLoop) "Local") false false))
  ;[1 1 1] Cable attach and length
  (for _index_2 (range 0 (Variables|Default|GetNumberOfSplinePoints))
    (Variables|Default|SetIndexLoop2 _index_2)
    (Utilities|FlowControl|Sequence
      (:then_0
        (Transformation|AttachComponentToComponent (Variables|/Game/Blueprints/Ruins/BP_powerline.BP_powerline_C|GetCable1 (Utilities|Array|Get(acopy) (Variables|Default|GetAllChildActorsOfPowerline) (Variables|Default|GetIndexLoop2))) (Variables|/Game/Blueprints/Ruins/BP_powerline.BP_powerline_C|GetConnection1 (Utilities|Array|Get(acopy) (Variables|Default|GetAllChildActorsOfPowerline) (+ (Variables|Default|GetIndexLoop2) 1))) "None" "SnapToTarget" "SnapToTarget" "KeepWorld" true) ; Cable 1
        (Variables|/Script/CableComponent.CableComponent|SetCableLength (Variables|/Game/Blueprints/Ruins/BP_powerline.BP_powerline_C|GetCable1 (Utilities|Array|Get(acopy) (Variables|Default|GetAllChildActorsOfPowerline) (Variables|Default|GetIndexLoop2))) (+ (Math|Vector|VectorLength (- (Transformation|GetWorldLocation (Variables|/Game/Blueprints/Ruins/BP_powerline.BP_powerline_C|GetConnection1 (Utilities|Array|Get(acopy) (Variables|Default|GetAllChildActorsOfPowerline) (Variables|Default|GetIndexLoop2)))) (Transformation|GetWorldLocation (Variables|/Game/Blueprints/Ruins/BP_powerline.BP_powerline_C|GetConnection1 (Utilities|Array|Get(acopy) (Variables|Default|GetAllChildActorsOfPowerline) (+ (Variables|Default|GetIndexLoop2) 1)))))) (Math|Random|RandomFloatinRange 0.0 3e+01)))
        ;[1 1 1] Set end cable length to 0
        (Variables|/Script/CableComponent.CableComponent|SetCableLength (Variables|/Game/Blueprints/Ruins/BP_powerline.BP_powerline_C|GetCable1 (Utilities|Array|Get(acopy) (Variables|Default|GetAllChildActorsOfPowerline) (Variables|Default|GetNumberOfSplinePoints))) 0.0))
      (:then_1
        (Transformation|AttachComponentToComponent (Variables|/Game/Blueprints/Ruins/BP_powerline.BP_powerline_C|GetCable2 (Utilities|Array|Get(acopy) (Variables|Default|GetAllChildActorsOfPowerline) (Variables|Default|GetIndexLoop2))) (Variables|/Game/Blueprints/Ruins/BP_powerline.BP_powerline_C|GetConnection2 (Utilities|Array|Get(acopy) (Variables|Default|GetAllChildActorsOfPowerline) (+ (Variables|Default|GetIndexLoop2) 1))) "None" "SnapToTarget" "SnapToTarget" "KeepWorld" true) ; Cable 2
        (Variables|/Script/CableComponent.CableComponent|SetCableLength (Variables|/Game/Blueprints/Ruins/BP_powerline.BP_powerline_C|GetCable2 (Utilities|Array|Get(acopy) (Variables|Default|GetAllChildActorsOfPowerline) (Variables|Default|GetIndexLoop2))) (+ (Math|Vector|VectorLength (- (Transformation|GetWorldLocation (Variables|/Game/Blueprints/Ruins/BP_powerline.BP_powerline_C|GetConnection2 (Utilities|Array|Get(acopy) (Variables|Default|GetAllChildActorsOfPowerline) (Variables|Default|GetIndexLoop2)))) (Transformation|GetWorldLocation (Variables|/Game/Blueprints/Ruins/BP_powerline.BP_powerline_C|GetConnection2 (Utilities|Array|Get(acopy) (Variables|Default|GetAllChildActorsOfPowerline) (+ (Variables|Default|GetIndexLoop2) 1)))))) (Math|Random|RandomFloatinRange 0.0 3e+01)))
        (Variables|/Script/CableComponent.CableComponent|SetCableLength (Variables|/Game/Blueprints/Ruins/BP_powerline.BP_powerline_C|GetCable2 (Utilities|Array|Get(acopy) (Variables|Default|GetAllChildActorsOfPowerline) (Variables|Default|GetNumberOfSplinePoints))) 0.0)))))