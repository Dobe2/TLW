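; BP_oak_tree is a choppable oak tree that the player fells with the Interact input.
; Overlapping the ChopZone component enables input and prints a prompt; leaving it disables input.
; Interact applies a mass-independent force to Tree along the player controller's forward direction, then destroys ChopZone so it cannot be chopped again.
; The construction script sets rotation from random rotators and randomizes uniform scale for variety.
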(event OnComponentBeginOverlap(ChopZone)
  (params (OverlappedComponent :type Primitive%20Component%20Object%20Reference) (OtherActor :type Actor%20Object%20Reference) (OtherComp :type Primitive%20Component%20Object%20Reference) (OtherBodyIndex :type Integer) (bFromSweep :type Boolean) (SweepResult :type Hit%20Result%20Structure%20%28by%20ref%29))
  ;[1 1 1] Is the player in range
  (Input|EnableInput (Game|GetPlayerController 0))
  (Variables|Default|SetChopZoneIsActive true)
  (Development|PrintString "Can Chop (Interact)" true false "(R=0.562500,G=0.000000,B=0.018082,A=1.000000)"))

(event OnComponentEndOverlap(ChopZone)
  (params (OverlappedComponent :type Primitive%20Component%20Object%20Reference) (OtherActor :type Actor%20Object%20Reference) (OtherComp :type Primitive%20Component%20Object%20Reference) (OtherBodyIndex :type Integer))
  ;[1 1 1] Is the player in range
  (Input|DisableInput (Game|GetPlayerController 0))
  (Variables|Default|SetChopZoneIsActive false))

(event EventBeginPlay)

(event Collision|EventActorBeginOverlap
  (params (OtherActor :type Actor%20Object%20Reference))
  (Input|EnableInput 0))

(event EventTick
  (params (DeltaSeconds :type Float%20%28single-precision%29)))

(event Input|ActionEvents|InputActionInteract
  (params (Key :type Key%20Structure))
  ;[1 1 1] Commence chopping!
  (:Pressed
    (if (Variables|Default|GetChopZoneIsActive)
      (Physics|AddForce (Variables|Default|GetTree) (* (Math|Rotator|GetRotationXVector (Transformation|GetActorRotation (Game|GetPlayerController 0))) (Variables|Default|GetChop%20Force)) "None" true)
      (Components|DestroyComponent (Variables|Default|GetChop%20Zone)))))

(fn ConstructionScript
  (bind _returnvalue (Math|Random|RandomRotator false))
  (bind (_x _y) (Math|Rotator|BreakRotIntoAxes _returnvalue))
  ;[1 1 1] Random rotation
  (Transformation|SetActorRotation (Math|Conversions|RotationFromXVector _x))
  (Transformation|SetActorRotation (Math|Conversions|RotationFromXVector _y))
  ;[1 1 1] Random height
  (Transformation|SetActorScale3D (Math|Conversions|ToVector(Float) (.X (Math|Vector|BreakVector (Math|Vector|MakeVector (Math|Random|RandomFloatinRange 0.8 1.2) 0.0 0.0))))))