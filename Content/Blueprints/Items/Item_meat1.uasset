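; Meat item actor that removes itself from the world when the player comes near.
; Tick checks the player character's distance every frame and destroys the actor once it is within 1000 units, granting nothing.
; The PickUpZone overlap events are empty; disconnected leftover nodes hold an unused interact-to-pickup flow with input toggling, a CanPickup flag and debug prints.
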(event OnComponentBeginOverlap(PickUpZone)
  (params (OverlappedComponent :type Primitive%20Component%20Object%20Reference) (OtherActor :type Actor%20Object%20Reference) (OtherComp :type Primitive%20Component%20Object%20Reference) (OtherBodyIndex :type Integer) (bFromSweep :type Boolean) (SweepResult :type Hit%20Result%20Structure%20%28by%20ref%29))
  ;[1 1 1] Is the player in range
)

(event OnComponentEndOverlap(PickUpZone)
  (params (OverlappedComponent :type Primitive%20Component%20Object%20Reference) (OtherActor :type Actor%20Object%20Reference) (OtherComp :type Primitive%20Component%20Object%20Reference) (OtherBodyIndex :type Integer))
  ;[1 1 1] Is the player in range
)

(event EventBeginPlay)

(event Collision|EventActorBeginOverlap
  (params (OtherActor :type Actor%20Object%20Reference)))

(event EventTick
  (params (DeltaSeconds :type Float%20%28single-precision%29))
  (if (>= 1e+03 (Transformation|GetDistanceTo (Game|GetPlayerCharacter 0) 0))
    (Actor|DestroyActor)))

(event Input|ActionEvents|InputActionInteract
  (params (Key :type Key%20Structure)))

(fn ConstructionScript)